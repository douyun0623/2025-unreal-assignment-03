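; BP_UFO is a rideable UFO that puts the Granny character into flight when she touches it.
; On box overlap it casts to Granny, snaps itself onto her mesh and switches her movement mode to Flying.
; It makes her follow controller pitch and yaw instead of movement direction, sets OnUFO and clears JumpHigh.
; The file has no detach or dismount logic.
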(event `self.Box.OnComponentBeginOverlap`
  (params (OverlappedComponent :type "PrimitiveComponent Object Reference") (OtherActor :type "Actor Object Reference") (OtherComp :type "PrimitiveComponent Object Reference") (OtherBodyIndex :type Integer) (bFromSweep :type Boolean) (SweepResult :type "HitResult Structure (by ref)"))
  (bind _as_granny (`self.As Granny`))
  (bind _charactermovement (`Character.CharacterMovement` _as_granny))
  (bind _asgranny (cast `/Game/_TEST2/Granny` OtherActor))
  (bind _output_get (set `self.As Granny` _asgranny))
  (`self.K2_AttachToComponent` (`Character.Mesh` _output_get) "None" "SnapToTarget" "SnapToTarget" "SnapToTarget")
  (`CharacterMovementComponent.SetMovementMode` _charactermovement "MOVE_Flying" 0)
  (set `CharacterMovementComponent.bOrientRotationToMovement` false _charactermovement)
  (set `Pawn.bUseControllerRotationPitch` true _as_granny)
  (set `Pawn.bUseControllerRotationYaw` true _as_granny)
  (set `/Game/_TEST2/Granny.On UFO?` true _as_granny)
  (set `/Game/_TEST2/Granny.JumpHigh?` false _as_granny))

(fn `UserConstructionScript`)