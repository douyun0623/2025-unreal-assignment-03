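; BP_Zombie is a killable zombie actor that triggers the win state when the last one dies.
; Any damage subtracts from its Hp, and it destroys itself once Hp runs out.
; After each death it counts remaining BP_Zombie actors; if none are left, it shows the BP_Win widget and sets the Win flag on the Granny actor.
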(event `self.ReceiveAnyDamage`
  (params (Damage :type "Float (single-precision)") (DamageType :type "DamageType Object Reference") (InstigatedBy :type "Controller Object Reference") (DamageCauser :type "Actor Object Reference"))
  (bind _output_get (set `self.hp` (- (`self.hp`) Damage)))
  (if (< _output_get 0.1)
    (`self.K2_DestroyActor`)
    (bind _outactors (`GameplayStatics.GetAllActorsOfClass` "BP_Zombie_C"))
    (if (< (`KismetArrayLibrary.Array_Length` _outactors) 1)
      (bind _returnvalue (`|CreateWidget` "/Game/_TEST2/BP_Win.BP_Win_C"))
      (`UserWidget.AddToViewport` _returnvalue 0)
      (bind _returnvalue_2 (`GameplayStatics.GetActorOfClass` "/Game/_TEST2/Granny.Granny_C"))
      (set `/Game/_TEST2/Granny.Win?` true _returnvalue_2))))

(fn `UserConstructionScript`)